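; BP_FPSHud is the FPS game's HUD Blueprint that spawns the on-screen game UI.
; On BeginPlay it creates the WBP_FPSGUI and WBP_Reticle widgets, adds both to the viewport and sets game-only input on the first player controller.
; The FPS GUI widget is stored and exposed through GetFPSGUI, while a node to remove it is left unconnected.
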(event EventBeginPlay
  (Development|PrintString "Spawning Game GUI")
  (bind _returnvalue (UserInterface|CreateWidget "/Game/FPS/Blueprints/GUI/Game/WBP_FPSGUI.WBP_FPSGUI_C"))
  (bind _output_get (Variables|Default|SetFPSGUI _returnvalue))
  ;[1 1 1] Adds UI
  (UserInterface|Viewport|AddtoViewport _output_get 0)
  (bind _returnvalue_2 (UserInterface|CreateWidget "/Game/FPS/Blueprints/GUI/Game/WBP_Reticle.WBP_Reticle_C"))
  (UserInterface|Viewport|AddtoViewport _returnvalue_2 0)
  (Input|SetInputModeGameOnly (Game|GetPlayerController 0) false))

(fn ConstructionScript)

(fn GetFPSGUI
  (return (Variables|Default|GetFPSGUI)))