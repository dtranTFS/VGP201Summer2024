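; FPS game mode that runs a countdown and shows it on the player's HUD.
; BeginPlay prints a debug message and caches player 0's HUD as BP_FPSHud.
; Tick uses a one-second Delay to throttle decrementing Countdown, then passes the value to the HUD's FPS GUI timer.
; The file has no handling for the countdown reaching zero.
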(event EventBeginPlay
  (Development|PrintString "Spawning FPSGameMode" true true "(R=1.000000,G=0.000000,B=0.000000,A=1.000000)")
  (bind _asbp_fpshud (Utilities|Casting|CastToBP_FPSHud (HUD|GetHUD (Game|GetPlayerController 0))))
  (Variables|Default|SetFPSHud _asbp_fpshud))

(event EventTick
  (params (DeltaSeconds :type Float%20%28single-precision%29))
  (bind _fpshud (Variables|Default|GetFPSHud))
  (Utilities|FlowControl|Delay 1.0)
  (bind _result (Math|Integer|DecrementInt (Variables|Default|GetCountdown))
    (:%20%20
      (Utilities|IsValid _fpshud
        (:Is%20Valid
          (Default|SetTimer (Default|GetFPSGUI _fpshud) (Math|Conversions|ToInteger(Byte) (Utilities|String|ToString(Integer) _result))))))))

(fn ConstructionScript)