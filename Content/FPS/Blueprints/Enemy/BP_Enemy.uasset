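; BP_Enemy is a damageable FPS enemy that can be reset after death instead of being destroyed.
; AnyDamage feeds TakeDamage, which applies damage through ACHealthComponent, then either disables the enemy on death or prints its remaining health.
; SetEnabled toggles visibility and collision on a mesh passed in through Init.
; Reset restores full health and re-enables that mesh, so the same actor can be reused.
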(event Game|Damage|EventAnyDamage
  (params (Damage :type Float%20%28single-precision%29) (DamageType :type Damage%20Type%20Object%20Reference) (InstigatedBy :type Controller%20Object%20Reference) (DamageCauser :type Actor%20Object%20Reference))
  (CallFunction|TakeDamage Damage))

(fn ConstructionScript)

(fn Reset
  (Default|HealFull (Variables|Default|GetAC_HealthComponent))
  (CallFunction|SetEnabled true (Variables|Default|GetMesh)))

(fn SetEnabled
  (params (IsActive :type Boolean) (Mesh :type Primitive%20Component%20Object%20Reference))
  (Rendering|SetVisibility Mesh IsActive false)
  (if IsActive
    (Collision|SetCollisionEnabled Mesh "QueryAndPhysics")
    (else
      (Collision|SetCollisionEnabled Mesh "NoCollision"))))

(fn Init
  (params (Mesh :type Primitive%20Component%20Object%20Reference))
  (Variables|Default|SetMesh Mesh))

(fn TakeDamage
  (params (Damage%20Amount :type Float%20%28double-precision%29))
  (bind _ac_healthcomponent (Variables|Default|GetAC_HealthComponent))
  (Default|Damage _ac_healthcomponent Damage%20Amount)
  (if (Default|IsDead _ac_healthcomponent)
    (CallFunction|SetEnabled false (Variables|Default|GetMesh))
    (else
      (Development|PrintString (Utilities|String|ToString(Float) (Default|GetHealth _ac_healthcomponent))))))